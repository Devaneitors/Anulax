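; Ranged enemy pawn that shoots Bullet_BP projectiles at the player, driven by an AI controller Blackboard.
; BeginPlay stores the player in the Blackboard; Sphere overlap sets IsAtacking and stops movement, while overlap end only clears HasCollided.
; Attack spawns a player-aimed bullet, then, gated by CanAttack, plays AttackNS and a Timeline-driven Body yaw animation.
; Tick fakes sprite-style flipping by toggling Left/Right visibility from the player's relative Y position.
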(event OnComponentBeginOverlap(Sphere)
  (params (OverlappedComponent :type Primitive%20Component%20Object%20Reference) (OtherActor :type Actor%20Object%20Reference) (OtherComp :type Primitive%20Component%20Object%20Reference) (OtherBodyIndex :type Integer) (bFromSweep :type Boolean) (SweepResult :type Hit%20Result%20Structure%20%28by%20ref%29))
  ;[1 1 1] alcanza al player y le pega, si se aleja vuelve a perseguirle
  (Utilities|Casting|CastToBP_ThirdPersonCharacter OtherActor)
  (Variables|Default|SethasCollided true)
  (AI|Components|Blackboard|SetValueasBool (AI|GetBlackboard (AI|GetAIController self)) (Utilities|Name|MakeLiteralName "IsAtacking") true)
  (Components|Movement|StopMovementImmediately (Variables|Character|GetCharacterMovement)))

(event OnComponentEndOverlap(Sphere)
  (params (OverlappedComponent :type Primitive%20Component%20Object%20Reference) (OtherActor :type Actor%20Object%20Reference) (OtherComp :type Primitive%20Component%20Object%20Reference) (OtherBodyIndex :type Integer))
  ;[1 1 1] alcanza al player y le pega, si se aleja vuelve a perseguirle
  (Utilities|Casting|CastToBP_ThirdPersonCharacter OtherActor)
  (Variables|Default|SethasCollided false))

(event Custom|Attack
  (bind _self self)
  (bind _body (Variables|Default|GetBody))
  (bind _returnvalue (Transformation|GetActorLocation _self))
  (bind _relativerotation (Variables|/Script/Engine.SceneComponent|GetRelativeRotation _body))
  ;[1 1 1] disparo
  (Game|SpawnActorfromClass "/Game/EnemiesIA/Bullet_BP.Bullet_BP_C" (Math|Transform|MakeTransform _returnvalue (Math|Rotator|FindLookatRotation _returnvalue (Transformation|GetActorLocation (Game|GetPlayerCharacter 0))) "1.000000,1.000000,1.000000") "Undefined" "MultiplyWithRoot" 0 _self)
  ;[1 1 1] Animacion ataque
  (if (Variables|Default|GetCan%20Attack)
    (Components|Activation|Activate (Variables|Default|GetAttack%20NS) true)
    (Variables|Default|SetCan%20Attack (Variables|Default|GetCan%20Attack))
    (bind _newtrack_0 (Timeline|Timeline PlayFromStart)
      (:Update
        (Transformation|SetRelativeRotation _body (Math|Rotator|MakeRotator (.roll _relativerotation) (.pitch _relativerotation) _newtrack_0) false false))
      (:Finished
        (Utilities|FlowControl|Delay 0.3)
        (Variables|Default|SetCan%20Attack true)))))

(event EventBeginPlay
  (bind _self self)
  (bind _returnvalue (AI|GetAIController _self))
  (bind _returnvalue_2 (AI|GetBlackboard _returnvalue))
  ;[1 1 1] setea el backboard
  (AI|Components|Blackboard|SetValueasBool _returnvalue_2 (Utilities|Name|MakeLiteralName "IsAtacking") false)
  (AI|Components|Blackboard|SetValueasObject _returnvalue_2 (Utilities|Name|MakeLiteralName "Player") (Game|GetPlayerCharacter 0)))

(event EventTick
  (params (DeltaSeconds :type Float%20%28single-precision%29))
  (bind _returnvalue (Game|GetPlayerCharacter 0))
  (bind _self self)
  (bind _returnvalue_2 (Transformation|GetActorLocation _returnvalue))
  (bind _returnvalue_3 (Transformation|GetActorLocation _self))
  (bind _returnvalue_4 (> (.y _returnvalue_2) (.y _returnvalue_3)))
  ;[1 1 1] flip del enemigo por posición del jugador
  (Rendering|SetVisibility (Variables|Default|GetRight) _returnvalue_4 true)
  (Rendering|SetVisibility (Variables|Default|GetLeft) (not _returnvalue_4) true))

(fn ConstructionScript)