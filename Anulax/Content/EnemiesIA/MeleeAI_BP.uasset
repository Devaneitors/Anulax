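; Melee enemy that chases the player, attacks up close and is destroyed when its hits run out.
; The Sphere overlap sets the AI Blackboard's attack flag.
; Attack waits briefly, plays an effect, damages the player inside Attackspace, then clears the flag if they left, running a Body yaw Timeline.
; Tick fakes a side-view flip by toggling Left/Right visibility and moving Attackspace toward the player's side on Y.
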(event OnComponentBeginOverlap(Sphere)
  (params (OverlappedComponent :type Primitive%20Component%20Object%20Reference) (OtherActor :type Actor%20Object%20Reference) (OtherComp :type Primitive%20Component%20Object%20Reference) (OtherBodyIndex :type Integer) (bFromSweep :type Boolean) (SweepResult :type Hit%20Result%20Structure%20%28by%20ref%29))
  ;[1 1 1] alcanza al player y le pega, si se aleja vuelve a perseguirle
  (Utilities|Casting|CastToBP_ThirdPersonCharacter OtherActor)
  (Variables|Default|SethasCollided true)
  (AI|Components|Blackboard|SetValueasBool (AI|GetBlackboard (AI|GetAIController self)) (Utilities|Name|MakeLiteralName "IsAtacking") true))

(event OnComponentBeginOverlap(attackspace)
  (params (OverlappedComponent :type Primitive%20Component%20Object%20Reference) (OtherActor :type Actor%20Object%20Reference) (OtherComp :type Primitive%20Component%20Object%20Reference) (OtherBodyIndex :type Integer) (bFromSweep :type Boolean) (SweepResult :type Hit%20Result%20Structure%20%28by%20ref%29))
  ;[1 1 1] el jugador está dentro del rango del ataque
  (Utilities|Casting|CastToBP_ThirdPersonCharacter OtherActor)
  (Variables|Default|SetisAttackRange true))

(event OnComponentEndOverlap(attackspace)
  (params (OverlappedComponent :type Primitive%20Component%20Object%20Reference) (OtherActor :type Actor%20Object%20Reference) (OtherComp :type Primitive%20Component%20Object%20Reference) (OtherBodyIndex :type Integer))
  ;[1 1 1] el jugador está dentro del rango del ataque
  (Utilities|Casting|CastToBP_ThirdPersonCharacter OtherActor)
  (Variables|Default|SetisAttackRange false))

(event OnComponentEndOverlap(Sphere)
  (params (OverlappedComponent :type Primitive%20Component%20Object%20Reference) (OtherActor :type Actor%20Object%20Reference) (OtherComp :type Primitive%20Component%20Object%20Reference) (OtherBodyIndex :type Integer))
  ;[1 1 1] alcanza al player y le pega, si se aleja vuelve a perseguirle
  (Utilities|Casting|CastToBP_ThirdPersonCharacter OtherActor)
  (Variables|Default|SethasCollided false))

(event Custom|Death
  ;[1 1 1] Muerte
  (Actor|DestroyActor))

(event Custom|Damaged
  (bind _vidaactual (Variables|Default|GetVidaActual))
  ;[1 1 1] ha recibido daño, y si este daño le deja en 0 vidas o menos le mata
  (Math|Integer|DecrementInt _vidaactual
    (:%20%20
      (Development|PrintString (Utilities|String|ToString(Integer) _vidaactual))
      (if (<= _vidaactual 0)
        (CallFunction|Death)))))

(event Custom|Attack
  (bind _body (Variables|Default|GetBody))
  (bind _relativerotation (Variables|/Script/Engine.SceneComponent|GetRelativeRotation _body))
  ;[1 1 1] alcanza al player y le pega, si se aleja vuelve a perseguirle
  (Utilities|FlowControl|Delay 0.3)
  (if (Variables|Default|GetCan%20Attack)
    (Components|Activation|Activate (Variables|Default|GetAttack%20NS) true)
    (Variables|Default|SetCan%20Attack (Variables|Default|GetCan%20Attack))
    (if (Variables|Default|GetisAttackRange)
      (bind _asbp_third_person_character (Utilities|Casting|CastToBP_ThirdPersonCharacter (Game|GetPlayerCharacter 0)))
      ;[1 1 1] Animacion ataque
      (Default|Damaged _asbp_third_person_character)
      (if (not (Variables|Default|GethasCollided))
        (AI|Components|Blackboard|SetValueasBool (AI|GetBlackboard (AI|GetAIController self)) (Utilities|Name|MakeLiteralName "IsAtacking") false :!label _label)
        (bind _newtrack_0 (Timeline|Timeline PlayFromStart)
          (:Update
            (Transformation|SetRelativeRotation _body (Math|Rotator|MakeRotator (.roll _relativerotation) (.pitch _relativerotation) _newtrack_0) false false))
          (:Finished
            (Utilities|FlowControl|Delay 0.3)
            (Variables|Default|SetCan%20Attack true))))
      (else
        (goto _label)))))

(event EventBeginPlay
  (bind _self self)
  (bind _returnvalue (AI|GetAIController _self))
  (bind _returnvalue_2 (AI|GetBlackboard _returnvalue))
  ;[1 1 1] setea el backboard
  (AI|Components|Blackboard|SetValueasBool _returnvalue_2 (Utilities|Name|MakeLiteralName "IsAtacking") false)
  (AI|Components|Blackboard|SetValueasObject _returnvalue_2 (Utilities|Name|MakeLiteralName "Player") (Game|GetPlayerCharacter 0))
  (Rendering|SetVisibility (Variables|Default|GetLeft) false true)
  (Variables|Default|SetVidaActual (Variables|Default|GetVidaMax)))

(event EventTick
  (params (DeltaSeconds :type Float%20%28single-precision%29))
  (bind _returnvalue (Game|GetPlayerCharacter 0))
  (bind _self self)
  (bind _attackspace (Variables|Default|Getattackspace))
  (bind _returnvalue_2 (Transformation|GetActorLocation _returnvalue))
  (bind _returnvalue_3 (Transformation|GetActorLocation _self))
  (bind _returnvalue_4 (> (.y _returnvalue_2) (.y _returnvalue_3)))
  ;[1 1 1] flip del enemigo por posición del jugador
  (Rendering|SetVisibility (Variables|Default|GetRight) _returnvalue_4 true)
  (Rendering|SetVisibility (Variables|Default|GetLeft) (not _returnvalue_4) true)
  (if _returnvalue_4
    (Transformation|SetRelativeLocation _attackspace "0.000000,70.000000,0.000000" false false)
    (else
      (Transformation|SetRelativeLocation _attackspace "0.000000,-70.000000,0.000000" false false))))

(fn ConstructionScript)

(fn Dead)