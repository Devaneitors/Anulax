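; Boss-related briefcase actor (Maletin) that acts as an emergence point for melee enemies.
; On BeginPlay, SpawnMelees gathers every existing MeleeAI_BP in the level once and teleports them one by one to the briefcase's location.
; A Delay wired back into an IndexMelee check forms the timed loop, so enemies are relocated at fixed intervals rather than newly spawned.
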(event Custom|SpawnMelees
  (bind _indexmelee (Variables|Default|GetIndexMelee))
  (bind _outactors (Actor|GetAllActorsOfClass "/Game/EnemiesIA/MeleeAI_BP.MeleeAI_BP_C"))
  (if (< _indexmelee (Utilities|Array|Length _outactors)) :!label _label
    (Utilities|FlowControl|Delay 2.0)
    (Transformation|SetActorLocation (Utilities|Array|Get(acopy) _outactors _indexmelee) (Transformation|GetActorLocation self) false true)
    (Math|Integer|IncrementInt _indexmelee
      (:%20%20
        (goto _label)))))

(event EventBeginPlay
  (CallFunction|SpawnMelees))

(event Collision|EventActorBeginOverlap
  (params (OtherActor :type Actor%20Object%20Reference)))

(event EventTick
  (params (DeltaSeconds :type Float%20%28single-precision%29)))

(fn ConstructionScript)