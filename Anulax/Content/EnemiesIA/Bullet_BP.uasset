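; Bullet actor, apparently fired by enemies, that damages the third-person player character on contact.
; Its capsule overlap reacts only to other capsule components, ignores actors tagged Enemy, calls Damaged on BP_ThirdPersonCharacter, and destroys the bullet for any non-Enemy hit.
; Tick sets LifeSpan to a constant before subtracting delta time, so the timed self-destroy does not accumulate across frames.
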(event OnComponentBeginOverlap(Capsule)
  (params (OverlappedComponent :type Primitive%20Component%20Object%20Reference) (OtherActor :type Actor%20Object%20Reference) (OtherComp :type Primitive%20Component%20Object%20Reference) (OtherBodyIndex :type Integer) (bFromSweep :type Boolean) (SweepResult :type Hit%20Result%20Structure%20%28by%20ref%29))
  (Utilities|Casting|CastToCapsuleComponent OtherComp)
  (if (not (Actor|ActorHasTag OtherActor "Enemy"))
    (bind _asbp_third_person_character (Utilities|Casting|CastToBP_ThirdPersonCharacter OtherActor)
      (:then
        (Default|Damaged _asbp_third_person_character))
      (:CastFailed
        _))
    (Actor|DestroyActor)))

(event EventBeginPlay)

(event Collision|EventActorBeginOverlap
  (params (OtherActor :type Actor%20Object%20Reference)))

(event EventTick
  (params (DeltaSeconds :type Float%20%28single-precision%29))
  (Variables|Default|SetLifeSpan 1e+01)
  (bind _output_get (Variables|Default|SetLifeSpan (- (Variables|Default|GetLifeSpan) DeltaSeconds)))
  (if (<= _output_get 0.0)
    (Actor|DestroyActor)))

(fn ConstructionScript)