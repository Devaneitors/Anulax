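; Door Blueprint that acts as a level exit once every melee and ranger AI enemy is gone.
; When the third-person player character overlaps its Box, it counts all MeleeAI_BP and RangerAI_BP actors in the level.
; If none remain, it switches on the current level name to open the next room, with the third room leading to ThirdPersonMap.
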(event OnComponentBeginOverlap(Box)
  (params (OverlappedComponent :type Primitive%20Component%20Object%20Reference) (OtherActor :type Actor%20Object%20Reference) (OtherComp :type Primitive%20Component%20Object%20Reference) (OtherBodyIndex :type Integer) (bFromSweep :type Boolean) (SweepResult :type Hit%20Result%20Structure%20%28by%20ref%29))
  (Utilities|Casting|CastToBP_ThirdPersonCharacter OtherActor)
  (bind _outactors (Actor|GetAllActorsOfClass "/Game/EnemiesIA/MeleeAI_BP.MeleeAI_BP_C"))
  (bind _outactors_2 (Actor|GetAllActorsOfClass "/Game/EnemiesIA/RangerAI_BP.RangerAI_BP_C"))
  (if (<= (+ (Utilities|Array|Length _outactors) (Utilities|Array|Length _outactors_2)) 0)
    (bind _returnvalue (Game|GetCurrentLevelName true))
    (switch string _returnvalue
      (:Room_1
        (Game|OpenLevel(byName) "Room_2"))
      (:Room_2
        (Game|OpenLevel(byName) "Room_3"))
      (:Room_3
        (Game|OpenLevel(byName) "ThirdPersonMap")))))

(event EventBeginPlay)

(event Collision|EventActorBeginOverlap
  (params (OtherActor :type Actor%20Object%20Reference)))

(event EventTick
  (params (DeltaSeconds :type Float%20%28single-precision%29)))

(fn ConstructionScript)